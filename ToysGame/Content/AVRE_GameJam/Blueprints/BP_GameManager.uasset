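; Game manager that spawns corona enemies in waves of one at a time from an array of scene spawners.
; From BeginPlay, a Delay loop waits random seconds and calls SpawnCorona on a random spawner until NumberOfSpawns or GameOver.
; Short delays avoid repeating the last spawner by shifting at array ends; a middle repeat stops the loop.
; Loop exit shows the win message through BP_AlertWindow, even on GameOver.
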(event EventBeginPlay
  (bind _coronaspawnsinscene (Variables|CoronaSpawnController|GetCoronaSpawnsInScene))
  (bind _returnvalue (Utilities|Array|Length _coronaspawnsinscene))
  (bind _returnvalue_2 (- _returnvalue 1))
  (bind _returnvalue_3 (Math|Random|RandomIntegerinRange 0 _returnvalue_2))
  (if (> (Utilities|Array|Length (Variables|CoronaSpawnController|GetCoronaSpawnsInScene)) 0)
    (if (and (> (Variables|CoronaSpawnController|GetNumberOfSpawns) (Variables|CoronaSpawnController|GetCurrentSpawns)) (not (Variables|Default|GetGameOver))) :!label _label
      (Development|PrintString (Utilities|String|ToString(Integer) (Variables|CoronaSpawnController|GetCurrentSpawns)))
      (Variables|CoronaSpawnController|SetCurrentSpawns (+ (Variables|CoronaSpawnController|GetCurrentSpawns) 1))
      ;[1 1 1] Wait the random time and spawn in a random spawner
      (bind _output_get (Variables|CoronaSpawnController|SetCurrentDelay (Math|Random|RandomIntegerinRange 0 (Variables|CoronaSpawnController|GetMaxSpawnDelay))))
      (Utilities|FlowControl|Delay (Math|Conversions|ToFloat(Integer) _output_get))
      (if (> (Variables|CoronaSpawnController|GetCurrentDelay) 1)
        (bind _output_get_2 (Variables|CoronaSpawnController|SetLastSpawner _returnvalue_3))
        (Default|SpawnCorona (Utilities|Array|Get(acopy) (Variables|CoronaSpawnController|GetCoronaSpawnsInScene) _output_get_2)) ; Normal spawn
        (goto _label)
        (else
          (bind _output_get_3 (Variables|Default|SetCurrentSpawner _returnvalue_3))
          (if (== _output_get_3 (Variables|CoronaSpawnController|GetLastSpawner))
            (if (== (Variables|CoronaSpawnController|GetLastSpawner) (- (Utilities|Array|Length (Variables|CoronaSpawnController|GetCoronaSpawnsInScene)) 1))
              (bind _output_get_4 (Variables|CoronaSpawnController|SetLastSpawner (- (Variables|CoronaSpawnController|GetLastSpawner) 1)))
              (Default|SpawnCorona (Utilities|Array|Get(acopy) (Variables|CoronaSpawnController|GetCoronaSpawnsInScene) _output_get_4)) ; Spawn in a diferent spawn for don't collapse
              (goto _label)
              (elif (== (Variables|CoronaSpawnController|GetLastSpawner) 0)
                (bind _output_get_5 (Variables|CoronaSpawnController|SetLastSpawner (+ (Variables|CoronaSpawnController|GetLastSpawner) 1)))
                (Default|SpawnCorona (Utilities|Array|Get(acopy) (Variables|CoronaSpawnController|GetCoronaSpawnsInScene) _output_get_5)) ; Spawn in a diferent spawn for dont collapse
                (goto _label)))
            (else
              (bind _output_get_6 (Variables|CoronaSpawnController|SetLastSpawner (Variables|Default|GetCurrentSpawner)))
              (Default|SpawnCorona (Utilities|Array|Get(acopy) (Variables|CoronaSpawnController|GetCoronaSpawnsInScene) _output_get_6)) ; Normal spawn
              (goto _label)))))
      (else
        (bind _returnvalue_4 (Actor|GetActorOfClass "/Game/AVRE_GameJam/Blueprints/BP_AlertWindow.BP_AlertWindow_C"))
        (Default|ShowCanvas _returnvalue_4 "YOU WIN! 
Press Y or B to restart the game")))
    (else
      (Development|PrintString "FILL CORONA SPAWNS IN SCENE"))))

(event Collision|EventActorBeginOverlap
  (params (OtherActor :type Actor%20Object%20Reference)))

(event EventTick
  (params (DeltaSeconds :type Float%20%28single-precision%29)))

(fn ConstructionScript)