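; BP_Corona is the virus actor in a game jam game where it threatens the city.
; Its Hit event branches on the other actor's class through casts.
; Hitting BP_City plays a sound, destroys the virus and shows the game-over restart prompt through the BP_AlertWindow found in the level.
; Hitting BP_IceTruck plays a sound and destroys only the truck, while any other actor just prints a debug string.
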(event EventBeginPlay)

(event Collision|EventActorBeginOverlap
  (params (OtherActor :type Actor%20Object%20Reference)))

(event EventTick
  (params (DeltaSeconds :type Float%20%28single-precision%29)))

(event Collision|EventHit
  (params (MyComp :type Primitive%20Component%20Object%20Reference) (Other :type Actor%20Object%20Reference) (OtherComp :type Primitive%20Component%20Object%20Reference) (bSelfMoved :type Boolean) (HitLocation :type Vector :default "0, 0, 0") (HitNormal :type Vector :default "0, 0, 0") (NormalImpulse :type Vector :default "0, 0, 0") (Hit :type Hit%20Result%20Structure%20%28by%20ref%29))
  (Utilities|Casting|CastToBP_City Other
    (:then
      (Audio|PlaySoundatLocation "/Engine/VREditor/Sounds/UI/Flashlight_Switch.Flashlight_Switch" (Transformation|GetWorldLocation (Variables|Default|GetSphere)) "0, 0, 0" 1.0 1.0 0.0 0 0 0) ; Sound when the virus hit the city
      (Actor|DestroyActor)
      (bind _returnvalue (Actor|GetActorOfClass "/Game/AVRE_GameJam/Blueprints/BP_AlertWindow.BP_AlertWindow_C"))
      (Default|ShowCanvas _returnvalue "Game over 
Press Y or B to restart the game"))
    (:CastFailed
      (bind _asbp_ice_truck (Utilities|Casting|CastToBP_IceTruck Other)
        (:then
          (Audio|PlaySoundatLocation "/Engine/VREditor/Sounds/UI/Laser_Push.Laser_Push" (Transformation|GetWorldLocation (Variables|Default|GetSphere)) "0, 0, 0" 1.0 1.0 0.0 0 0 0) ; Sound when we stop the virus
          (Actor|DestroyActor _asbp_ice_truck))
        (:CastFailed
          (Development|PrintString "HITTED A STRANGE OBJECT"))))))

(fn ConstructionScript)