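; BP_Ball is a physics ball that is thrown by impulse when its trigger activates, then can be scored or reset.
; Throw applies the configured damping and impulse once until reset, and Tick changes damping once the moving, unscored ball slows below a speed threshold.
; Score brakes the ball with high damping.
; ResetBall clears the state flags, uses extreme damping to hold it, and returns it to the location saved in the Construction Script.
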(event EventBeginPlay)

(event EventTick
  (params (DeltaSeconds :type Float%20%28single-precision%29))
  (if (Variables|Throw|GetbThrowed)
    (bind _returnvalue (Physics|GetPhysicsLinearVelocity (Variables|Default|GetSphereMesh) "None"))
    (if (Math|Boolean|ANDBoolean (<= (Math|Vector|VectorLength _returnvalue) 3e+02) (> (Math|Vector|VectorLength _returnvalue) 0.0) (not (Variables|Throw|GetbSlowed)) (not (Variables|Throw|GetbScored)))
      (Development|PrintString "SLOWED" true true "(R=1.000000,G=0.000000,B=0.007289,A=1.000000)" 5.0)
      (Class|PrimitiveComponent|SetLinearDamping (Variables|Default|GetSphereMesh) 0.5)
      (Class|PrimitiveComponent|SetAngularDamping (Variables|Default|GetSphereMesh) 0.5)
      (Variables|Throw|SetbSlowed true))))

(event EventTriggerActivated
  (if (not (Variables|Throw|GetbThrowed))
    (CallFunction|Throw)))

(fn ConstructionScript
  (Variables|Default|SetInitialLocation (Transformation|GetWorldLocation (Variables|Default|GetSphereMesh))))

(fn Throw
  (Class|PrimitiveComponent|SetLinearDamping (Variables|Default|GetSphereMesh) (Variables|Friction|GetLinearDamping))
  (Class|PrimitiveComponent|SetAngularDamping (Variables|Default|GetSphereMesh) (Variables|Friction|GetAngularDamping))
  (Physics|AddImpulse (Variables|Default|GetSphereMesh) (Variables|Throw|GetImpulseForce) "None" false)
  (Variables|Throw|SetbThrowed true))

(fn Score
  (Variables|Throw|SetbScored true)
  (Class|PrimitiveComponent|SetLinearDamping (Variables|Default|GetSphereMesh) 1e+01)
  (Class|PrimitiveComponent|SetAngularDamping (Variables|Default|GetSphereMesh) 1e+01))

(fn ResetBall
  (Variables|Throw|SetbSlowed false)
  (Variables|Throw|SetbScored false)
  (Variables|Throw|SetbThrowed false)
  (Class|PrimitiveComponent|SetLinearDamping (Variables|Default|GetSphereMesh) 1e+05)
  (Class|PrimitiveComponent|SetAngularDamping (Variables|Default|GetSphereMesh) 1e+06)
  (Transformation|SetWorldLocation (Variables|Default|GetSphereMesh) (Variables|Default|GetInitialLocation) false false)
  (Development|PrintString "RESET"))