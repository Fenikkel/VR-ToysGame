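; BP_leverSwitch is a physics-driven two-position lever that triggers another actor when flipped.
; Each tick it reads the handle's pitch in actor space and sets the physics constraint's angular target to -45 or 45 degrees, pulling the handle toward whichever side it leans.
; When that side changes, it updates SwitchOn and sends TriggerActivatedMessage to TriggerableActor via BPI_Triggerable, in either direction, printing a warning if the interface is missing.
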(event EventBeginPlay)

(event Collision|EventActorBeginOverlap
  (params (OtherActor :type Actor%20Object%20Reference)))

(event EventTick
  (params (DeltaSeconds :type Float%20%28single-precision%29))
  (bind _returnvalue (Transformation|GetActorTransform))
  (bind _handle (Variables|Default|GetHandle))
  (bind _returnvalue_2 (Transformation|GetWorldRotation _handle))
  (bind _returnvalue_3 (Math|Transform|InverseTransformRotation _returnvalue _returnvalue_2))
  (bind _pitch (Math|Rotator|BreakRotator _returnvalue_3))
  (bind _returnvalue_4 (< _pitch 0.0))
  (Class|PhysicsConstraintComponent|SetAngularOrientationTarget (Variables|Default|GetPhysicsConstraint) (Math|Rotator|MakeRotator 0.0 (select _returnvalue_4 -45.0 45.0) 0.0))
  (if (Math|Boolean|NotEqual(Boolean) (Variables|Default|GetSwitchOn) _returnvalue_4)
    (Variables|Default|SetSwitchOn _returnvalue_4)
    (if (Utilities|DoesObjectImplementInterface (Variables|Default|GetTriggerableActor) "/Game/ToysGame/BluePrints/BPI_Triggerable.BPI_Triggerable_C")
      (Class|BPITriggerable|TriggerActivated(Message) (Variables|Default|GetTriggerableActor))
      (else
        (Development|PrintString "The triggered actor with the lever doesn't implement BPI_Triggerable" true true "(R=1.000000,G=0.016048,B=0.000000,A=1.000000)" 1e+01)))))

(fn ConstructionScript)