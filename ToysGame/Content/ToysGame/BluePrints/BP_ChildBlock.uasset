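; A toy letter block that BP_MotionController can pick up and drop.
; The construction script picks a random index and applies materials from LettersMaterials to six of the mesh's material slots.
; Pickup turns off physics simulation and attaches the root to the given component, keeping its world transform.
; Drop restores physics and detaches the block where it is.
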(event EventBeginPlay)

(event Collision|EventActorBeginOverlap
  (params (OtherActor :type Actor%20Object%20Reference)))

(event EventTick
  (params (DeltaSeconds :type Float%20%28single-precision%29)))

(event EventPickup
  (params (AttachTo :type Scene%20Component%20Object%20Reference))
  (Physics|SetSimulatePhysics (Variables|Debug|GetStaticMeshComponent) false)
  (Transformation|AttachComponentToComponent (VehicleSound|GetRootComponent) AttachTo "None" "KeepWorld" "KeepWorld" "KeepWorld" false))

(event EventDrop
  (Physics|SetSimulatePhysics (Variables|Debug|GetStaticMeshComponent) true)
  (Transformation|DetachFromActor "KeepWorld" "KeepWorld" "KeepWorld"))

(fn ConstructionScript
  (Variables|Default|SetRandomIndex (Math|Random|RandomIntegerinRange 0 3))
  (Rendering|Material|SetMaterial (Variables|Debug|GetStaticMeshComponent) 1 (Utilities|Array|Get(acopy) (Variables|Default|GetLettersMaterials) (Variables|Default|GetRandomIndex)))
  (Rendering|Material|SetMaterial (Variables|Debug|GetStaticMeshComponent) 2 (Utilities|Array|Get(acopy) (Variables|Default|GetLettersMaterials) (Variables|Default|GetRandomIndex)))
  (Rendering|Material|SetMaterial (Variables|Debug|GetStaticMeshComponent) 3 (Utilities|Array|Get(acopy) (Variables|Default|GetLettersMaterials) (Variables|Default|GetRandomIndex)))
  (Rendering|Material|SetMaterial (Variables|Debug|GetStaticMeshComponent) 4 (Utilities|Array|Get(acopy) (Variables|Default|GetLettersMaterials) (Variables|Default|GetRandomIndex)))
  (Rendering|Material|SetMaterial (Variables|Debug|GetStaticMeshComponent) 5 (Utilities|Array|Get(acopy) (Variables|Default|GetLettersMaterials) (Variables|Default|GetRandomIndex)))
  (Rendering|Material|SetMaterial (Variables|Debug|GetStaticMeshComponent) 6 (Utilities|Array|Get(acopy) (Variables|Default|GetLettersMaterials) (Variables|Default|GetRandomIndex))))