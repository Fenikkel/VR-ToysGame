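; BP_BuildingObject is a placement preview that follows a motion controller's aim and spawns the selected buildable.
; The construction script sets the preview mesh and scale from parallel arrays indexed by CurrentBuildable.
; Each tick, a line trace positions it and a bounds-sized box trace permits building only on unobstructed floor, identified by static mesh, swapping materials accordingly.
; BuildObject spawns the matching class at the preview transform if allowed, then destroys the preview regardless.
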(event Custom|BuildObject
  (bind _classesofbuildables (Variables|Buildables|GetClassesOfBuildables))
  (bind _returnvalue (Utilities|Array|Length _classesofbuildables))
  (if (Variables|BuildData|GetCanBuild)
    (if (and (< (Variables|ExposedOnSpawn|GetCurrentBuildable) _returnvalue) (> _returnvalue 0))
      (Game|SpawnActorfromClass (Utilities|Array|Get(acopy) (Variables|Buildables|GetClassesOfBuildables) (Variables|ExposedOnSpawn|GetCurrentBuildable)) (Transformation|GetWorldTransform (Variables|Default|GetPreviewMesh)) "AlwaysSpawn" 0 0)
      (else
        (Development|PrintString "Index Out Of Bounds -> ListOfBuildeables in BP_BuildingObject" true true "(R=1.000000,G=0.144247,B=0.194014,A=1.000000)" 4.0)))
    (Actor|DestroyActor)
    (else
      (Actor|DestroyActor))))

(event Custom|LoopBreaker
  (Utilities|Array|ForEachLoopwithBreak (stale EventTick _outhits_2)) ; enters at Break
)

(event EventBeginPlay)

(event EventTick
  (params (DeltaSeconds :type Float%20%28single-precision%29))
  (bind _currentcontroller (Variables|ExposedOnSpawn|GetCurrentController))
  (bind _currentcontroller_2 (Variables|ExposedOnSpawn|GetCurrentController))
  (bind _motioncontroller (Variables|/Game/VirtualRealityBP/Blueprints/BP_MotionController.BP_MotionController_C|GetMotionController _currentcontroller))
  (bind _motioncontroller_2 (Variables|/Game/VirtualRealityBP/Blueprints/BP_MotionController.BP_MotionController_C|GetMotionController _currentcontroller_2))
  (bind _returnvalue (Transformation|GetWorldLocation _motioncontroller_2))
  (bind (_outhit _returnvalue_2) (Collision|LineTraceByChannel _returnvalue (+ _returnvalue (* (Math|Vector|GetForwardVector _motioncontroller_2) (Variables|BuildData|GetBuildingRange))) "TraceTypeQuery1" false 0 "ForOneFrame"))
  (if _returnvalue_2
    (bind _asstatic_mesh_actor (Utilities|Casting|CastToStaticMeshActor (.HitActor (Collision|BreakHitResult _outhit)))
      (:then
        (if (== (Variables|/Script/Engine.StaticMeshComponent|GetStaticMesh (Variables|/Script/Engine.StaticMeshActor|GetStaticMeshComponent _asstatic_mesh_actor)) (Variables|FloorData|GetFloorStaticMesh))
          (bind (_outhits _returnvalue_3) (Class|KismetSystemLibrary|BoxTraceMultiforObjects (+ (.Location (Collision|BreakHitResult _outhit)) (Math|Vector|MakeVector 0.0 0.0 (* (.Z (Math|Vector|BreakVector (.BoxExtent (Math|BoxSphereBounds|BreakBoxSphereBounds (StaticMesh|GetBounds (Variables|/Script/Engine.StaticMeshComponent|GetStaticMesh (Variables|Default|GetPreviewMesh))))))) (.Z (Math|Vector|BreakVector (Transformation|GetWorldScale (Variables|Default|GetPreviewMesh))))))) (+ (.Location (Collision|BreakHitResult _outhit)) (Math|Vector|MakeVector 0.0 0.0 (* (.Z (Math|Vector|BreakVector (.BoxExtent (Math|BoxSphereBounds|BreakBoxSphereBounds (StaticMesh|GetBounds (Variables|/Script/Engine.StaticMeshComponent|GetStaticMesh (Variables|Default|GetPreviewMesh))))))) (.Z (Math|Vector|BreakVector (Transformation|GetWorldScale (Variables|Default|GetPreviewMesh))))))) (* (.BoxExtent (Math|BoxSphereBounds|BreakBoxSphereBounds (StaticMesh|GetBounds (Variables|/Script/Engine.StaticMeshComponent|GetStaticMesh (Variables|Default|GetPreviewMesh))))) (Transformation|GetWorldScale (Variables|Default|GetPreviewMesh))) "0, 0, 0" (Utilities|Array|MakeArray "ObjectTypeQuery2" "ObjectTypeQuery4" "ObjectTypeQuery3" "ObjectTypeQuery1") false 0 "ForOneFrame" true))
          (if _returnvalue_3
            (bind _asstatic_mesh_actor_2 (Utilities|Casting|CastToStaticMeshActor (.HitActor (Collision|BreakHitResult (Utilities|Array|Get(acopy) _outhits))))
              (:then
                (if (and (== (Variables|/Script/Engine.StaticMeshComponent|GetStaticMesh (Variables|/Script/Engine.StaticMeshActor|GetStaticMeshComponent _asstatic_mesh_actor_2)) (Variables|FloorData|GetFloorStaticMesh)) (== (Utilities|Array|Length _outhits) 1))
                  ;[1 1 1] If we are hitting the floor and nothing else, spawn in the hit floor plus mesh offset
                  (Transformation|SetActorLocation (+ (.Location (Collision|BreakHitResult _outhit)) (Math|Vector|MakeVector 0.0 0.0 (* (.Z (Math|Vector|BreakVector (.BoxExtent (Math|BoxSphereBounds|BreakBoxSphereBounds (StaticMesh|GetBounds (Variables|/Script/Engine.StaticMeshComponent|GetStaticMesh (Variables|Default|GetPreviewMesh))))))) (.Z (Math|Vector|BreakVector (Transformation|GetWorldScale (Variables|Default|GetPreviewMesh))))))) false false :!label _label)
                  (CallFunction|SetBuildableZoneMaterial)
                  (Variables|BuildData|SetCanBuild true)
                  (else
                    ;[1 1 1] If we are hitting the floor but the static mesh is colliding with another object
                    (Transformation|SetActorLocation (+ (.Location (Collision|BreakHitResult _outhit)) (Math|Vector|MakeVector 0.0 0.0 (* (.Z (Math|Vector|BreakVector (.BoxExtent (Math|BoxSphereBounds|BreakBoxSphereBounds (StaticMesh|GetBounds (Variables|/Script/Engine.StaticMeshComponent|GetStaticMesh (Variables|Default|GetPreviewMesh))))))) (.Z (Math|Vector|BreakVector (Transformation|GetWorldScale (Variables|Default|GetPreviewMesh))))))) false false :!label _label_2)
                    (CallFunction|SetUnbuildableZoneMaterial)
                    (Variables|BuildData|SetCanBuild false))))
              (:CastFailed
                (goto _label_2)))
            (else
              (goto _label)))
          (else
            (bind (_outhits_2 _returnvalue_4) (Class|KismetSystemLibrary|BoxTraceMultiforObjects (.Location (Collision|BreakHitResult _outhit)) (.Location (Collision|BreakHitResult _outhit)) (* (.BoxExtent (Math|BoxSphereBounds|BreakBoxSphereBounds (StaticMesh|GetBounds (Variables|/Script/Engine.StaticMeshComponent|GetStaticMesh (Variables|Default|GetPreviewMesh))))) (Transformation|GetWorldScale (Variables|Default|GetPreviewMesh))) "0, 0, 0" (Utilities|Array|MakeArray "ObjectTypeQuery2" "ObjectTypeQuery4" "ObjectTypeQuery3" "ObjectTypeQuery1") false 0 "ForOneFrame" true :!label _label_3))
            (if _returnvalue_4
              (Variables|FloorData|SetFloorFound false)
              (bind _array_element (Utilities|Array|ForEachLoopwithBreak _outhits_2)
                (:LoopBody
                  (bind _asstatic_mesh_actor_3 (Utilities|Casting|CastToStaticMeshActor (.HitActor (Collision|BreakHitResult _array_element))))
                  (if (== (Variables|/Script/Engine.StaticMeshComponent|GetStaticMesh (Variables|/Script/Engine.StaticMeshActor|GetStaticMeshComponent _asstatic_mesh_actor_3)) (Variables|FloorData|GetFloorStaticMesh))
                    (Variables|FloorData|SetFloorPosition (.Location (Math|Transform|BreakTransform (Transformation|GetActorTransform _asstatic_mesh_actor_3))))
                    (Variables|FloorData|SetFloorFound true)
                    (CallFunction|LoopBreaker)))
                (:Completed
                  ;[1 1 1] True if the object is hitting the floor
                  (if (Variables|FloorData|GetFloorFound)
                    ;[1 1 1] If we are hitting something different to the floor but the the object collide with the floor, spawn in the hit but with the floor offset
                    (Transformation|SetActorLocation (Math|Vector|MakeVector (.X (Math|Vector|BreakVector (.Location (Collision|BreakHitResult _outhit)))) (.Y (Math|Vector|BreakVector (.Location (Collision|BreakHitResult _outhit)))) (+ (* (.Z (Math|Vector|BreakVector (.BoxExtent (Math|BoxSphereBounds|BreakBoxSphereBounds (StaticMesh|GetBounds (Variables|/Script/Engine.StaticMeshComponent|GetStaticMesh (Variables|Default|GetPreviewMesh))))))) (.Z (Math|Vector|BreakVector (Transformation|GetWorldScale (Variables|Default|GetPreviewMesh))))) (.Z (Math|Vector|BreakVector (Variables|FloorData|GetFloorPosition))))) false false)
                    (CallFunction|SetUnbuildableZoneMaterial)
                    (Variables|BuildData|SetCanBuild false)
                    (else
                      ;[1 1 1] If we are hitting something different to the floor and the the object don't collide with the floor, spawn in the hit
                      (Transformation|SetActorLocation (.Location (Collision|BreakHitResult _outhit)) false false)
                      (CallFunction|SetUnbuildableZoneMaterial)
                      (Variables|BuildData|SetCanBuild false)))))))))
      (:CastFailed
        (goto _label_3)))
    (else
      ;[1 1 1] If we don't hit nothing, spawn in the BuildingRange
      (Transformation|SetActorLocation (+ (Math|Vector|MakeVector 0.0 0.0 (* (.Z (Math|Vector|BreakVector (.BoxExtent (Math|BoxSphereBounds|BreakBoxSphereBounds (StaticMesh|GetBounds (Variables|/Script/Engine.StaticMeshComponent|GetStaticMesh (Variables|Default|GetPreviewMesh))))))) (.Z (Math|Vector|BreakVector (Transformation|GetWorldScale (Variables|Default|GetPreviewMesh)))))) (+ (Transformation|GetWorldLocation _motioncontroller) (* (Math|Vector|GetForwardVector _motioncontroller) (Variables|BuildData|GetBuildingRange)))) false false)
      (CallFunction|SetUnbuildableZoneMaterial)
      (Variables|BuildData|SetCanBuild false))))

(fn ConstructionScript
  (bind _staticmeshofbuildables (Variables|Buildables|GetStaticMeshOfBuildables))
  (bind _classesofbuildables (Variables|Buildables|GetClassesOfBuildables))
  (bind _staticmeshofbuildables_2 (Variables|Buildables|GetStaticMeshOfBuildables))
  (bind _previewscaleofbuildables (Variables|Buildables|GetPreviewScaleOfBuildables))
  (bind _currentbuildable (Variables|ExposedOnSpawn|GetCurrentBuildable))
  (bind _returnvalue (Utilities|Array|Length _classesofbuildables))
  (bind _returnvalue_2 (Utilities|Array|Length _staticmeshofbuildables_2))
  (bind _returnvalue_3 (Utilities|Array|Length _previewscaleofbuildables))
  (bind _output (Utilities|Array|Get(acopy) _staticmeshofbuildables _currentbuildable))
  ;[1 1 1] Remember
  (if (and (< (Variables|ExposedOnSpawn|GetCurrentBuildable) _returnvalue_2) (> _returnvalue_2 0))
    (Utilities|IsValid _output
      (:Is%20Valid
        (Components|StaticMesh|SetStaticMesh (Variables|Default|GetPreviewMesh) _output)
        (if (and (< (Variables|ExposedOnSpawn|GetCurrentBuildable) _returnvalue_3) (> _returnvalue_3 0))
          (Transformation|SetRelativeScale3D (Variables|Default|GetPreviewMesh) (Utilities|Array|Get(acopy) (Variables|Buildables|GetPreviewScaleOfBuildables) (Variables|ExposedOnSpawn|GetCurrentBuildable)))
          (if (not (and (== (Utilities|Array|Length (Variables|Buildables|GetStaticMeshOfBuildables)) _returnvalue) (== _returnvalue (Utilities|Array|Length (Variables|Buildables|GetPreviewScaleOfBuildables)))))
            (Development|PrintString "PreviewScaleOfBuildeables, StaticMeshComponentsOfBuildables and ClassesOfBuildables in BP_BuildingObject must have the same size." true true "(R=1.000000,G=0.144247,B=0.194014,A=1.000000)" 4.0))
          (else
            (Development|PrintString "Index Out Of Bounds ->PreviewScaleOfBuildebles in BP_BuildingObject" true true "(R=1.000000,G=0.144247,B=0.194014,A=1.000000)" 4.0))))
      (:Is%20Not%20Valid
        (Development|PrintString "INVALID STATIC MESH")))
    (else
      (Development|PrintString "Index Out Of Bounds ->StaticMeshComponentsOfBuildables in BP_BuildingObject" true true "(R=1.000000,G=0.144247,B=0.194014,A=1.000000)" 4.0))))

(fn SetBuildableZoneMaterial
  (for _index (range 0 (Rendering|Material|GetNumMaterials (Variables|Default|GetPreviewMesh)))
    (Rendering|Material|SetMaterial (Variables|Default|GetPreviewMesh) _index (Variables|Default|GetBuildableZoneMaterial))))

(fn SetUnbuildableZoneMaterial
  (for _index (range 0 (Rendering|Material|GetNumMaterials (Variables|Default|GetPreviewMesh)))
    (Rendering|Material|SetMaterial (Variables|Default|GetPreviewMesh) _index (Variables|Default|GetUnbuildableZoneMaterial))))