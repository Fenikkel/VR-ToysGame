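; A physical VR push button that motion controllers press to trigger a linked actor through BPI_Triggerable.
; On overlap it tracks the controller each tick, projecting its movement onto the button's up axis and clamping it to drive button travel.
; At full travel it raises the dynamic material's Glow and sends the trigger message.
; After a press or controller exit it interpolates back to rest, then restores the initial glow.
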(event OnComponentBeginOverlap(Button)
  (params (OverlappedComponent :type Primitive%20Component%20Object%20Reference) (OtherActor :type Actor%20Object%20Reference) (OtherComp :type Primitive%20Component%20Object%20Reference) (OtherBodyIndex :type Integer) (bFromSweep :type Boolean) (SweepResult :type Hit%20Result%20Structure%20%28by%20ref%29))
  (if (and (not (Variables|Default|GetbIsTracking)) (not (Variables|Default|GetbIsReturning)))
    (bind _asbp_motion_controller (Utilities|Casting|CastToBP_MotionController OtherActor))
    (Variables|Default|SetCurrentMC (Variables|/Game/VirtualRealityBP/Blueprints/BP_MotionController.BP_MotionController_C|GetMotionController _asbp_motion_controller))
    (Variables|Default|SetbIsTracking true)
    (Variables|Default|SetMCInitialLoaction (Transformation|GetWorldLocation (Variables|Default|GetCurrentMC)))))

(event OnComponentEndOverlap(Button)
  (params (OverlappedComponent :type Primitive%20Component%20Object%20Reference) (OtherActor :type Actor%20Object%20Reference) (OtherComp :type Primitive%20Component%20Object%20Reference) (OtherBodyIndex :type Integer))
  (bind _asbp_motion_controller (Utilities|Casting|CastToBP_MotionController OtherActor))
  (if (== (Variables|/Game/VirtualRealityBP/Blueprints/BP_MotionController.BP_MotionController_C|GetMotionController _asbp_motion_controller) (Variables|Default|GetCurrentMC))
    (Variables|Default|SetbIsTracking false)
    (Variables|Default|SetbIsReturning true)))

(event Custom|Fully%20Pressed
  (Rendering|Material|SetScalarParameterValue (Variables|Default|GetMaterialInstance%20Button) "Glow" (Variables|ButtonVariables|GetGlowIntensity) :!class /Script/Engine.MaterialInstanceDynamic)
  (Variables|Default|SetbIsTracking false)
  (Variables|Default|SetbIsReturning true)
  (if (Utilities|DoesObjectImplementInterface (Variables|Triggerable|GetTriggerableActor) "/Game/ToysGame/BluePrints/BPI_Triggerable.BPI_Triggerable_C")
    (Class|BPITriggerable|TriggerActivated(Message) (Variables|Triggerable|GetTriggerableActor))
    (else
      (Development|PrintString "The triggered actor with the button doesn't implement BPI_Triggerable" true true "(R=1.000000,G=0.016048,B=0.000000,A=1.000000)" 1e+01))))

(event EventBeginPlay
  (bind _returnvalue (Rendering|Material|CreateDynamicMaterialInstance (Variables|Default|GetButton) 0 "/Game/ToysGame/Material/M_VRButtonButton.M_VRButtonButton" "None" :!class /Script/Engine.PrimitiveComponent)) ; We create a material instance for edit one of his variables later
  (bind _output_get (Variables|Default|SetMaterialInstance%20Button _returnvalue))
  (bind _returnvalue_2 (Rendering|Material|GetScalarParameterValue _output_get "Glow" :!class /Script/Engine.MaterialInstanceDynamic))
  (Variables|Default|SetInitialGlowValue _returnvalue_2)
  (Variables|Default|SetButtonInitiaLocation (Transformation|GetWorldLocation (Variables|Default|GetButton))))

(event EventTick
  (params (DeltaSeconds :type Float%20%28single-precision%29))
  (if (Variables|Default|GetbIsTracking)
    (Variables|Default|SetCurrentButtonTravel (Math|Float|Clamp(Float) (Math|Float|Absolute(Float) (Math|Vector|VectorLength (Math|Vector|ProjectVectorontoVector (- (Transformation|GetWorldLocation (Variables|Default|GetCurrentMC)) (Variables|Default|GetMCInitialLoaction)) (Math|Vector|GetUpVector (Variables|Default|GetButton))))) (Variables|ButtonVariables|GetMinimumTravel) (Variables|ButtonVariables|GetMaximumTravel)))
    (bind _output_get (Variables|Default|SetButtonCurrentLocation (- (Variables|Default|GetButtonInitiaLocation) (* (Math|Vector|GetUpVector (Variables|Default|GetButton)) (Variables|Default|GetCurrentButtonTravel)))))
    (Transformation|SetWorldLocation (Variables|Default|GetButton) _output_get false false)
    (if (>= (Variables|Default|GetCurrentButtonTravel) (Variables|ButtonVariables|GetMaximumTravel))
      (CallFunction|FullyPressed))
    (elif (Variables|Default|GetbIsReturning)
      (bind _output_get_2 (Variables|Default|SetButtonCurrentLocation (Math|Interpolation|VInterpTo (Variables|Default|GetButtonCurrentLocation) (Variables|Default|GetButtonInitiaLocation) (Utilities|Time|GetWorldDeltaSeconds) (Variables|ButtonVariables|GetReturnSpeed))))
      (Transformation|SetWorldLocation (Variables|Default|GetButton) _output_get_2 false false)
      (if (Class|KismetMathLibrary|EqualExactlyVectorVector (Variables|Default|GetButtonCurrentLocation) (Variables|Default|GetButtonInitiaLocation))
        (Variables|Default|SetbIsReturning false)
        (Rendering|Material|SetScalarParameterValue (Variables|Default|GetMaterialInstance%20Button) "Glow" (Variables|Default|GetInitialGlowValue) :!class /Script/Engine.MaterialInstanceDynamic)
        (Development|PrintString (Utilities|String|ToString(Float) (Variables|Default|GetInitialGlowValue)) true true "(R=0.000000,G=0.660000,B=1.000000,A=1.000000)" 5.0)))))

(fn ConstructionScript)